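; BP_Bed is the level's ending trigger, a bed the player cat reaches once it has enough score.
; On box overlap by BP_PlayerCha it compares the GameInstance score, cached at BeginPlay, against RequireScore.
; If met, it stops the player's movement, changes the cat state, then after timed delays fades out and removes the HUD.
; It then shows the END widget and enables the mouse cursor.
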(event OnComponentBeginOverlap(Box)
  (params (OverlappedComponent :type Primitive%20Component%20Object%20Reference) (OtherActor :type Actor%20Object%20Reference) (OtherComp :type Primitive%20Component%20Object%20Reference) (OtherBodyIndex :type Integer) (bFromSweep :type Boolean) (SweepResult :type Hit%20Result%20Structure%20%28by%20ref%29))
  (bind _asbp_player_cha (Utilities|Casting|CastToBP_PlayerCha OtherActor))
  (if (>= (Variables|/Game/BP/BP_GameInstance.BP_GameInstance_C|GetScore (Variables|Default|GetGameInstance)) (Variables|Default|GetRequireScore))
    (Components|Movement|StopMovementImmediately (Pawn|GetMovementComponent _asbp_player_cha))
    (Utilities|FlowControl|Delay 0.5)
    (Variables|/Game/BP/BP_PlayerCha.BP_PlayerCha_C|SetCatState _asbp_player_cha "NewEnumerator2")
    (Utilities|FlowControl|Delay 4.0)
    (Class|UserWidget|PlayAnimationForward (Variables|/Game/BP/BP_PlayerCha.BP_PlayerCha_C|GetPlayerHUD _asbp_player_cha) (Variables|/Game/UserInterface/Player_HUD.Player_HUD_C|GetFadeOut (Variables|/Game/BP/BP_PlayerCha.BP_PlayerCha_C|GetPlayerHUD _asbp_player_cha)) 1.0 false)
    (Widget|RemovefromParent (Variables|/Game/BP/BP_PlayerCha.BP_PlayerCha_C|GetPlayerHUD _asbp_player_cha))
    (bind _returnvalue (UserInterface|CreateWidget "/Game/UserInterface/END.END_C" (Game|GetPlayerController 0)))
    (UserInterface|Viewport|AddtoViewport _returnvalue 0)
    (Variables|/Script/Engine.PlayerController|SetbShowMouseCursor (Game|GetPlayerController 0) true)))

(event EventBeginPlay
  (bind _asbp_game_instance (Utilities|Casting|CastToBP_GameInstance (Game|GetGameInstance)))
  (Variables|Default|SetGameInstance _asbp_game_instance))

(event Collision|EventActorBeginOverlap
  (params (OtherActor :type Actor%20Object%20Reference)))

(event EventTick
  (params (DeltaSeconds :type Float%20%28single-precision%29)))

(fn ConstructionScript)