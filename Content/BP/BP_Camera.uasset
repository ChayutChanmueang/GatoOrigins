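; BP_Camera is a side-view follow camera actor that makes itself the view target and tracks the player character's SideViewCameraComponent.
; On BeginPlay it snaps to that component and scales CameraLag into a small per-tick lerp alpha.
; Each tick it eases toward the component, clamps X between minimum and maximum bounds, floors Z at CameraZOffset and holds Y fixed.
; Older follow and look-at experiments remain unconnected.
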(event EventBeginPlay
  (Game|Player|SetViewTargetwithBlend (Game|GetPlayerController 0) self 0.0 "VTBlend_Linear" 0.0 false)
  (bind _asbp_player_cha (Utilities|Casting|CastToBP_PlayerCha (Game|GetPlayerCharacter 0)))
  (Variables|Default|SetPlayer _asbp_player_cha)
  (Transformation|SetActorLocation (Transformation|GetWorldLocation (Variables|/Game/BP/BP_PlayerCha.BP_PlayerCha_C|GetSideViewCameraComponent (Variables|Default|GetPlayer))) false false)
  (Variables|Default|SetCameraLag (* (Variables|Default|GetCameraLag) 0.01)))

(event Collision|EventActorBeginOverlap
  (params (OtherActor :type Actor%20Object%20Reference)))

(event EventTick
  (params (DeltaSeconds :type Float%20%28single-precision%29))
  (bind _returnvalue (Transformation|GetActorLocation))
  (bind _cameralag (Variables|Default|GetCameraLag))
  (bind _player (Variables|Default|GetPlayer))
  (bind _sideviewcameracomponent (Variables|/Game/BP/BP_PlayerCha.BP_PlayerCha_C|GetSideViewCameraComponent _player))
  (bind _returnvalue_2 (Transformation|GetWorldLocation _sideviewcameracomponent))
  (bind _returnvalue_3 (Math|Vector|Lerp(Vector) _returnvalue _returnvalue_2 _cameralag))
  (bind (_x _y _z) (Math|Vector|BreakVector _returnvalue_3))
  (Variables|Default|SetXPosition _x)
  (Variables|Default|SetZPosition _z)
  (Utilities|FlowControl|Sequence
    (:then_0
      (if (<= (Variables|Default|GetXPosition) (Variables|Default|GetCameraMinX))
        (Variables|Default|SetXPosition (Variables|Default|GetCameraMinX))))
    (:then_1
      (if (>= (Variables|Default|GetXPosition) (Variables|Default|GetCameraMaxX))
        (Variables|Default|SetXPosition (Variables|Default|GetCameraMaxX))))
    (:then_2
      (if (<= (Variables|Default|GetZPosition) (Variables|Default|GetCameraZOffset))
        (Variables|Default|SetZPosition (Variables|Default|GetCameraZOffset))))
    (:then_3
      (Transformation|SetActorLocation (Math|Vector|MakeVector (Variables|Default|GetXPosition) 1e+03 (Variables|Default|GetZPosition)) false false))))

(fn ConstructionScript)