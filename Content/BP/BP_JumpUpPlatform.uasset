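; BP_JumpUpPlatform is a sprite platform that the player character can pass through, named for jumping up through it.
; When BP_PlayerCha enters the Box trigger, the PaperSprite's collision is switched off and a Hit flag is set.
; When the player leaves the Box, collision returns as query-only after a short delay and the flag clears.
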(event OnComponentBeginOverlap(Box)
  (params (OverlappedComponent :type Primitive%20Component%20Object%20Reference) (OtherActor :type Actor%20Object%20Reference) (OtherComp :type Primitive%20Component%20Object%20Reference) (OtherBodyIndex :type Integer) (bFromSweep :type Boolean) (SweepResult :type Hit%20Result%20Structure%20%28by%20ref%29))
  (Utilities|Casting|CastToBP_PlayerCha OtherActor)
  (Collision|SetCollisionEnabled (Variables|Default|GetPaperSprite) "NoCollision")
  (Variables|Default|SetHit true))

(event OnComponentEndOverlap(Box)
  (params (OverlappedComponent :type Primitive%20Component%20Object%20Reference) (OtherActor :type Actor%20Object%20Reference) (OtherComp :type Primitive%20Component%20Object%20Reference) (OtherBodyIndex :type Integer))
  (Utilities|Casting|CastToBP_PlayerCha OtherActor)
  (if (Variables|Default|GetHit)
    (Utilities|FlowControl|Delay 0.5)
    (Collision|SetCollisionEnabled (Variables|Default|GetPaperSprite) "QueryOnly")
    (Variables|Default|SetHit false)))

(event EventBeginPlay)

(event Collision|EventActorBeginOverlap
  (params (OtherActor :type Actor%20Object%20Reference)))

(event EventTick
  (params (DeltaSeconds :type Float%20%28single-precision%29)))

(fn ConstructionScript)