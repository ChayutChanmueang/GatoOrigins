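; BP_LevelChanger is a trigger actor that moves the player to another level once the score is high enough.
; It caches BP_GameInstance on BeginPlay, then checks its Score against RequireScore when BP_PlayerCha overlaps the Box.
; If the requirement is met it opens the level given by LevelName, first zeroing the Score when ResetScoreAfterStage is set.
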(event OnComponentBeginOverlap(Box)
  (params (OverlappedComponent :type Primitive%20Component%20Object%20Reference) (OtherActor :type Actor%20Object%20Reference) (OtherComp :type Primitive%20Component%20Object%20Reference) (OtherBodyIndex :type Integer) (bFromSweep :type Boolean) (SweepResult :type Hit%20Result%20Structure%20%28by%20ref%29))
  (bind _level_name (Variables|Default|GetLevel%20Name))
  (Utilities|Casting|CastToBP_PlayerCha OtherActor)
  (if (>= (Variables|/Game/BP/BP_GameInstance.BP_GameInstance_C|GetScore (Variables|Default|GetGameInstance)) (Variables|Default|GetRequireScore))
    (if (Variables|Default|GetResetScoreAfterStage)
      (Variables|/Game/BP/BP_GameInstance.BP_GameInstance_C|SetScore (Variables|Default|GetGameInstance) 0)
      (Game|OpenLevel(byName) _level_name)
      (else
        (Game|OpenLevel(byName) _level_name)))))

(event EventBeginPlay
  (bind _asbp_game_instance (Utilities|Casting|CastToBP_GameInstance (Game|GetGameInstance)))
  (Variables|Default|SetGameInstance _asbp_game_instance))

(event Collision|EventActorBeginOverlap
  (params (OtherActor :type Actor%20Object%20Reference)))

(event EventTick
  (params (DeltaSeconds :type Float%20%28single-precision%29)))

(fn ConstructionScript)