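; Player cat character for a 2D Paper2D side-scroller, with movement, jump, pause, sleep and two mouse-triggered actions, attack and heart.
; Tick runs the cat state machine, where high anger speeds it up and inverts input, then updates flipbooks, facing and lives-based death screens.
; During an action, HitChecker uses flipbook frames to show an emote and pass the action to hitable objects overlapping the hit collider.
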(event Custom|Hit%20Checker
  (bind _catlider_hit_action (Variables|Default|GetCatlider_Hit_Action))
  (Utilities|FlowControl|Sequence
    (:then_0
      (if (== (Class|PaperFlipbookComponent|GetPlaybackPositioninFrames (Variables|Default|GetSprite)) 0)
        (Variables|Default|SetAbleToMove false)
        (Utilities|FlowControl|Sequence
          (:then_0
            (Rendering|SetVisibility (Variables|Default|GetEmotionSprite) true false)
            (Utilities|FlowControl|Delay 0.8)
            (Rendering|SetVisibility (Variables|Default|GetEmotionSprite) false false))
          (:then_1
            (if (not (Utilities|Enum|Equal(Enum) (Variables|Action_Catta|GetCat_Action) "NewEnumerator0"))
              (if (Utilities|Enum|Equal(Enum) (Variables|Action_Catta|GetCat_Action) "NewEnumerator1")
                (Rendering|Components|Sprite|SetSprite (Variables|Default|GetEmotionSprite) "/Game/Asset/emotion/atk_Sprite.atk_Sprite")
                (elif (Utilities|Enum|Equal(Enum) (Variables|Action_Catta|GetCat_Action) "NewEnumerator2")
                  (Rendering|Components|Sprite|SetSprite (Variables|Default|GetEmotionSprite) "/Game/Asset/emotion/heart_Sprite.heart_Sprite"))))))))
    (:then_1
      (if (== (Class|PaperFlipbookComponent|GetPlaybackPositioninFrames (Variables|Default|GetSprite)) 1)
        (Utilities|FlowControl|DoOnce false :!label _label
          (:Completed
            (Development|SetHiddeninGame _catlider_hit_action false false)
            (Utilities|FlowControl|Sequence
              (:then_0
                (for _array_element (Collision|GetOverlappingActors _catlider_hit_action 0 :!class /Script/Engine.PrimitiveComponent)
                  (bind _ashitable_objects_bp (Utilities|Casting|CastToHitable_Objects_BP _array_element))
                  (Default|InteractMyHeart _ashitable_objects_bp (Variables|Action_Catta|GetCat_Action))))
              (:then_2
                (Utilities|FlowControl|Delay 0.7)
                (goto _label Reset)))))))
    (:then_2
      (if (not (Audio|Components|Audio|IsPlaying (Variables|Default|GetSprite)))
        (Variables|Default|SetAbleToMove true)))))

(event Custom|UpdateAnimation
  (bind _sprite (Variables|Default|GetSprite))
  (bind _sprite_2 (Variables|Default|GetSprite))
  (bind _sprite_3 (Variables|Default|GetSprite))
  (bind _returnvalue (Transformation|GetWorldLocation _sprite))
  (bind _returnvalue_2 (Transformation|GetWorldLocation _sprite_2))
  (bind _returnvalue_3 (Transformation|GetWorldLocation _sprite_3))
  ;[1 1 1] Handle Animation
  (switch Utilities|FlowControl|Switch|SwitchonEnums_CatLevel (Variables|/Game/BP/BP_GameInstance.BP_GameInstance_C|GetCatLevel (Variables|Default|GetGameInstance))
    (:NewEnumerator1
      (switch Utilities|FlowControl|Switch|SwitchonEnums_CatState (Variables|Character|GetCatState)
        (:NewEnumerator0
          (if (Variables|Default|GetYawnStage)
            (Utilities|FlowControl|Sequence
              (:then_0
                (if (Variables|Action_Catta|GetIsHit)
                  (Sprite|SetFlipbook (Variables|Default|GetSprite) "/Game/Asset/FlipBook/catheart_thin1.catheart_thin1")
                  (else
                    (Sprite|SetFlipbook (Variables|Default|GetSprite) "/Game/Asset/FlipBook/Yawn.Yawn")))
                (Utilities|FlowControl|DoOnce false :!label _label
                  (:Completed
                    (Transformation|SetWorldLocation _sprite_2 (Math|Vector|MakeVector (.x _returnvalue_2) (.y _returnvalue_2) (- (.z _returnvalue_2) 1e+01)) false false))))
              (:then_1
                (Utilities|FlowControl|Delay 1.5)
                (Variables|Default|SetSitting true)
                (Variables|Default|SetYawnStage false)
                (Variables|Default|SetAbleToMove true)
                (Transformation|SetWorldLocation _sprite_3 (Math|Vector|MakeVector (.x _returnvalue_3) (.y _returnvalue_3) (+ (.z _returnvalue_3) 5.0)) false false)
                (goto _label Reset)))
            (elif (Variables|Default|GetSitting)
              (Sprite|SetFlipbook (Variables|Default|GetSprite) "/Game/Asset/FlipBook/Sit.Sit")
              (if (> (Math|Vector|VectorLength (Transformation|GetVelocity)) 0.0)
                (Variables|Default|SetSitting false)
                (Transformation|SetWorldLocation _sprite (Math|Vector|MakeVector (.x _returnvalue) (.y _returnvalue) (+ (.z _returnvalue) 5.0)) false false))
              (elif (AI|Components|NavMovement|IsFalling (Variables|Character|GetCharacterMovement))
                (Sprite|SetFlipbook (Variables|Default|GetSprite) "/Game/Asset/FlipBook/Jump_OnAir.Jump_OnAir")
                (else
                  (Sprite|SetFlipbook (Variables|Default|GetSprite) (select (> (Math|Vector|VectorLength (Transformation|GetVelocity)) 0.0) "/Game/Asset/FlipBook/Cat_walking.Cat_walking" "/Game/Asset/FlipBook/Cat_Idled.Cat_Idled")))))))
        (:NewEnumerator2
          (Utilities|FlowControl|Sequence
            (:then_0
              (Utilities|FlowControl|DoOnce false :!label _label_2
                (:Completed
                  (Sprite|SetFlipbook (Variables|Default|GetSprite) "/Game/Asset/FlipBook/Yawn.Yawn"))))
            (:then_1
              (Utilities|FlowControl|Delay 1.5)
              (Sprite|SetFlipbook (Variables|Default|GetSprite) "/Game/Asset/FlipBook/Sleep.Sleep")
              (Variables|Default|SetAbleToMove true)
              (if (> (Math|Vector|VectorLength (Transformation|GetVelocity)) 0.0)
                (Variables|Character|SetCatState "NewEnumerator0")
                (goto _label_2 Reset)))))))))

(event EventTick
  (params (DeltaSeconds :type Float%20%28single-precision%29))
  (bind _returnvalue (Pawn|GetController))
  (bind _returnvalue_2 (Pawn|GetController))
  (bind _charactermovement (Variables|Character|GetCharacterMovement))
  (bind _charactermovement_2 (Variables|Character|GetCharacterMovement))
  (Utilities|FlowControl|Sequence
    (:then_0
      ;[1 1 1] Handle Cat's State
      (switch Utilities|FlowControl|Switch|SwitchonEnums_CatState (Variables|Character|GetCatState)
        (:NewEnumerator0
          (if (>= (Variables|Character|GetAnger) 3e+01)
            (Variables|Character|SetCatState "NewEnumerator1")
            (Variables|Default|SetInvertInput true)
            (Variables|Default|SetAbleToMove true)))
        (:NewEnumerator1
          (Variables|/Script/Engine.CharacterMovementComponent|SetMaxWalkSpeed _charactermovement 6e+02)
          (Variables|/Script/Engine.CharacterMovementComponent|SetMaxAcceleration _charactermovement 2048.0)
          (if (> (Variables|Character|GetAnger) 0.0)
            (Variables|Character|SetAnger (- (Variables|Character|GetAnger) (Variables|Character|GetAngerReductionRate)))
            (else
              (Variables|Character|SetCatState "NewEnumerator0")
              (Variables|/Script/Engine.CharacterMovementComponent|SetMaxWalkSpeed _charactermovement_2 3e+02)
              (Variables|/Script/Engine.CharacterMovementComponent|SetMaxAcceleration _charactermovement_2 2048.0)
              (Variables|Default|SetInvertInput false)
              (Variables|Default|SetAbleToMove true))))))
    (:then_1
      ;[1 1 1] Tick - Updates animation
      (CallFunction|UpdateAnimation)
      (Math|Float|CompareFloat (.X (Math|Vector|BreakVector (Variables|/Script/Engine.MovementComponent|GetVelocity (Pawn|GetMovementComponent)))) 0.0
        (:>
          (Utilities|IsValid _returnvalue_2 :!label _label
            (:Is%20Valid
              (Pawn|SetControlRotation _returnvalue_2 (Math|Rotator|MakeRotator 0.0 0.0 0.0)))))
        (:==
          (if (Variables|Default|GetbisMovingRight)
            (goto _label)
            (else
              (Utilities|IsValid _returnvalue :!label _label_2
                (:Is%20Valid
                  (Pawn|SetControlRotation _returnvalue (Math|Rotator|MakeRotator 0.0 0.0 1.8e+02)))))))
        (:<
          (goto _label_2))))
    (:then_2
      (if (<= (Variables|Character|GetHealth) 0.0)
        (if (not (Variables|Default|GetIsDead))
          (bind _asbp_game_instance (Utilities|Casting|CastToBP_GameInstance (Game|GetGameInstance)))
          (if (<= (Variables|/Game/BP/BP_GameInstance.BP_GameInstance_C|GetLife _asbp_game_instance) 0)
            (Variables|Default|SetIsDead true)
            (bind _returnvalue_3 (UserInterface|CreateWidget "/Game/UserInterface/DeathScreen_OutofLife.DeathScreen_OutofLife_C" (Game|GetPlayerController 0)))
            (UserInterface|Viewport|AddtoViewport _returnvalue_3 0)
            (Variables|/Script/Engine.PlayerController|SetbShowMouseCursor (Game|GetPlayerController 0) true)
            (else
              (Variables|/Game/BP/BP_GameInstance.BP_GameInstance_C|SetLife _asbp_game_instance (- (Variables|/Game/BP/BP_GameInstance.BP_GameInstance_C|GetLife _asbp_game_instance) 1))
              (Variables|Default|SetIsDead true)
              (bind _returnvalue_4 (UserInterface|CreateWidget "/Game/UserInterface/DeathScreen.DeathScreen_C" (Game|GetPlayerController 0)))
              (UserInterface|Viewport|AddtoViewport _returnvalue_4 0)
              (Variables|/Script/Engine.PlayerController|SetbShowMouseCursor (Game|GetPlayerController 0) true))))))
    (:then_3
      (if (Variables|Default|GetYawnStage)
        (CallFunction|HitChecker)
        (else
          (Development|SetHiddeninGame (Variables|Default|GetCatlider_Hit_Action) true false))))))

(event EventBeginPlay
  (Class|ActorComponent|SetIsReplicated (Variables|Default|GetSprite) true)
  (bind _returnvalue (UserInterface|CreateWidget "/Game/UserInterface/Player_HUD.Player_HUD_C" (Game|GetPlayerController 0)))
  (UserInterface|Viewport|AddtoViewport _returnvalue 0)
  (Variables|Default|SetPlayerHUD _returnvalue)
  (bind _asbp_game_instance (Utilities|Casting|CastToBP_GameInstance (Game|GetGameInstance)))
  (Variables|Default|SetGameInstance _asbp_game_instance))

(event Input|ActionEvents|InputActionPause
  (params (Key :type Key%20Structure :default "None"))
  ;[1 1 1] Pause
  (:Pressed
    (if (Game|IsGamePaused)
      (Game|SetGamePaused false)
      (Widget|RemovefromParent (Variables|Default|GetPauseMenu))
      (Variables|/Script/Engine.PlayerController|SetbShowMouseCursor (Game|GetPlayerController 0) false)
      (else
        (Game|SetGamePaused true)
        (bind _returnvalue (UserInterface|CreateWidget "/Game/UserInterface/PauseMenu.PauseMenu_C" (Game|GetPlayerController 0)))
        (bind _output_get (Variables|Default|SetPauseMenu _returnvalue))
        (UserInterface|Viewport|AddtoViewport _output_get 0)
        (Variables|/Script/Engine.PlayerController|SetbShowMouseCursor (Game|GetPlayerController 0) true)))))

(event Input|ActionEvents|InputActionJump
  (params (Key :type Key%20Structure :default "None"))
  ;[1 1 1] Handle Jump
  (:Pressed
    (if (and (Variables|Default|GetAbleToMove) (Math|Boolean|NotEqual(Boolean) (Variables|Default|GetIsDead) true))
      (Character|Jump)))
  (:Released
    (Character|StopJumping)))

(event Input|AxisEvents|InputAxisMoveRight
  (params (AxisValue :type Float%20%28single-precision%29))
  ;[1 1 1] Handle movement
  (if (and (Variables|Default|GetAbleToMove) (Math|Boolean|NotEqual(Boolean) (Variables|Default|GetIsDead) true))
    (if (Variables|Default|GetInvertInput)
      (if (> AxisValue 0.0)
        (Variables|Default|SetbisMovingRight true)
        (elif (< AxisValue 0.0)
          (Variables|Default|SetbisMovingRight false)))
      (Pawn|Input|AddMovementInput "1.000000, 0, 0" (* -1 AxisValue) false)
      (else
        (if (> AxisValue 0.0)
          (Variables|Default|SetbisMovingRight true)
          (elif (< AxisValue 0.0)
            (Variables|Default|SetbisMovingRight false)))
        (Pawn|Input|AddMovementInput "1.000000, 0, 0" AxisValue false)))))

(event Input|KeyboardEvents|S
  (params (Key :type Key%20Structure :default "None"))
  (:Pressed
    (if (not (Variables|Default|GetYawnStage))
      (Variables|Default|SetYawnStage true)
      (Variables|Default|SetAbleToMove false))))

(event Input|KeyboardEvents|F
  (params (Key :type Key%20Structure :default "None"))
  (:Pressed
    (Variables|Character|SetCatState "NewEnumerator2")
    (Variables|Default|SetAbleToMove false)))

(event Input|KeyboardEvents|1
  (params (Key :type Key%20Structure :default "None"))
  (:Pressed
    (Variables|Action_Catta|SetCat_Action "NewEnumerator1")))

(event Input|KeyboardEvents|2
  (params (Key :type Key%20Structure :default "None"))
  (:Pressed
    (Variables|Action_Catta|SetCat_Action "NewEnumerator2")))

(event Input|MouseEvents|LeftMouseButton
  (params (Key :type Key%20Structure :default "None"))
  (:Pressed
    (Variables|Action_Catta|SetCat_Action "NewEnumerator1")
    (Variables|Default|SetYawnStage true)
    (Variables|Action_Catta|SetIsHit false)))

(event Input|MouseEvents|RightMouseButton
  (params (Key :type Key%20Structure :default "None"))
  (:Pressed
    (Variables|Action_Catta|SetCat_Action "NewEnumerator2")
    (Variables|Default|SetYawnStage true)
    (Variables|Action_Catta|SetIsHit true)))

(event Input|TouchEvents|InputTouch
  (params (Location :type Vector) (FingerIndex :type ETouchIndex%20Enum))
  ;[1 1 1] Handle Jump
  (:Pressed
    (if (and (Variables|Default|GetAbleToMove) (Math|Boolean|NotEqual(Boolean) (Variables|Default|GetIsDead) true))
      (Character|Jump)))
  (:Released
    (Character|StopJumping)))

(fn ConstructionScript)