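; Hittable fan mob with a 2D flipbook that reacts to the player's cat actions and drives a vertical hover on the player character.
; InteractMyHeart briefly swaps the idle flipbook for an action-specific reaction, then starts DelayHover, which toggles Hovering and resets the timer.
; While Hovering, Tick adds Z movement input scaled by Gravity and elapsed time, with a DoOnce that stops resetting at a time cap.
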(event Custom|ChangeMyHeart
  (params (NewParam :type CatAction%20Enum :default "NewEnumerator0"))
  (bind _fanmob_idle (Variables|Default|GetFanMob_Idle))
  (if (Utilities|Enum|Equal(Enum) NewParam "NewEnumerator2")
    (Sprite|SetFlipbook _fanmob_idle "/Game/Asset/FlipBook/FanMob_Inlove.FanMob_Inlove")
    (Utilities|FlowControl|Delay 1.0 :!label _label)
    (Sprite|SetFlipbook (Variables|Default|GetFanMob_Idle) "/Game/Asset/FlipBook/FanMob_Idle.FanMob_Idle")
    (elif (Utilities|Enum|Equal(Enum) NewParam "NewEnumerator1")
      (Sprite|SetFlipbook _fanmob_idle "/Game/Asset/FlipBook/FanMob_Guteak.FanMob_Guteak")
      (goto _label))))

(event Custom|Delay%20Hover
  (Variables|Default|SetHovering true)
  (Variables|Default|SetChildTime 0.0)
  (CallFunction|DelayHover)
  (Variables|Default|SetHovering false))

(event EventBeginPlay
  (|CallParentFunction) ; This node is disabled and will not be called.\nDrag off pins to build functionality.
)

(event Collision|EventActorBeginOverlap
  (params (OtherActor :type Actor%20Object%20Reference))
  (|CallParentFunction OtherActor) ; This node is disabled and will not be called.\nDrag off pins to build functionality.
)

(event EventTick
  (params (DeltaSeconds :type Float%20%28single-precision%29))
  (bind _asbp_player_cha (Utilities|Casting|CastToBP_PlayerCha (Game|GetPlayerCharacter 0)))
  (if (Variables|Default|GetHovering)
    (Utilities|FlowControl|DoOnce false :!label _label
      (:Completed
        (Variables|Default|SetChildTime (+ (* DeltaSeconds 1.0) (Variables|Default|GetChildTime)))
        (Class|PawnMovementComponent|AddInputVector (Variables|/Script/Engine.Character|GetCharacterMovement _asbp_player_cha) (+ (Math|Vector|MakeVector 0.0 0.0 0.0) (Math|Vector|MakeVector 0.0 0.0 (* 1 (* (Variables|Default|GetGravity) (Variables|Default|GetChildTime))))) false)
        (if (not (>= (Variables|Default|GetChildTime) 1e+01))
          (goto _label Reset))))))

(fn ConstructionScript
  (Rendering|Components|Sprite|SetSprite (Variables|Default|GetInputSprite) (Variables|Default|GetMySprite))
  (|CallParentFunction))

(fn InteractMyHeart
  (params (CatAction :type CatAction%20Enum :default "NewEnumerator0"))
  (Utilities|FlowControl|Sequence
    (:then_0
      (CallFunction|ChangeMyHeart CatAction))
    (:then_1
      (CallFunction|DelayHover))))