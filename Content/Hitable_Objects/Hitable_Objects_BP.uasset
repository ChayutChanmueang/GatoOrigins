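; Base-style Blueprint for a hitable object that glides toward a goal location, initially its own spawn position.
; MoveMyPoint offsets that goal and resets a timer, which Tick slowly increases and feeds as the lerp alpha from the current position, producing an eased move without sweep.
; Tick flags arrival within a small distance for CheckEndMove to report.
; InteractMyHeart takes a cat action but is an empty stub here.
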(event EventBeginPlay
  (Variables|Default|SetGoalLocation (Transformation|GetActorLocation)))

(event Collision|EventActorBeginOverlap
  (params (OtherActor :type Actor%20Object%20Reference)))

(event EventTick
  (params (DeltaSeconds :type Float%20%28single-precision%29))
  (bind _returnvalue (Transformation|GetActorLocation))
  (bind _goallocation (Variables|Default|GetGoalLocation))
  (Utilities|FlowControl|Sequence
    (:then_0
      (Math|Float|CompareFloat (Variables|Default|GetMyTime) 1.0
        (:>
          (Variables|Default|SetMyTime 0.02 :!label _label))
        (:==
          (goto _label))
        (:<
          _))
      (Transformation|SetActorLocation (Math|Vector|Lerp(Vector) _returnvalue _goallocation (Variables|Default|GetMyTime)) false false)
      (Variables|Default|SetMyTime (+ (Variables|Default|GetMyTime) (* DeltaSeconds 0.1)))
      (Variables|Default|SetIsStop (<= (Math|Vector|Distance(Vector) _returnvalue _goallocation) 0.1)))))

(fn ConstructionScript)

(fn MoveMyPoint
  (params (AddPosition :type Vector))
  (Variables|Default|SetGoalLocation (+ AddPosition (Variables|Default|GetGoalLocation)))
  (Variables|Default|SetMyTime 0.02))

(fn CheckEndMove
  (return (Variables|Default|GetIsStop)))

(fn InteractMyHeart
  (params (CatAction :type CatAction%20Enum :default "NewEnumerator0")))